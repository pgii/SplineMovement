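; CustomSpline_BP is a spline track actor that builds deformed meshes along an open or looping spline.
; Its Construction Script syncs SplinePointArray to the point count, then adds a spline mesh per segment using each point's mesh, width, height and roll.
; Optional point numbers and up-vector arrows visualize the points.
; AutoFillEmptyMesh acts as a self-resetting button, filling empty mesh slots with DefaultTrackMesh after segments are built.
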(event EventBeginPlay)

(fn ConstructionScript
  (bind _splinepointarray (Variables|Default|GetSplinePointArray))
  (bind _splinepointarray_2 (Variables|Default|GetSplinePointArray))
  (Utilities|FlowControl|Sequence
    (:then_0
      (Variables|Default|SetNumberOfSplinePoints (Spline|GetNumberOfSplinePoints (Variables|Default|GetSpline))))
    (:then_1
      (Math|Integer|CompareInt (Utilities|Array|Length _splinepointarray) (Variables|Default|GetNumberOfSplinePoints) :!label _label
        (:>
          (Utilities|Array|RemoveIndex _splinepointarray (Utilities|Array|LastIndex _splinepointarray))
          (goto _label))
        (:<
          (Utilities|Array|Add :TargetArray _splinepointarray)
          (goto _label))))
    (:then_2
      (for _index (range 0 (- (Variables|Default|GetNumberOfSplinePoints) (Math|Integer|SelectInt 1 2 (Variables|Default|GetLoopingTrack))))
        (Variables|Default|SetCurrentLoopIndex _index)
        (Spline|SetClosedLoop (Variables|Default|GetSpline) (Variables|Default|GetLoopingTrack) true)
        (CallFunction|InitSpline (Variables|Default|GetCurrentLoopIndex))
        (CallFunction|DrawPointNumber (Variables|Default|GetCurrentLoopIndex))
        (CallFunction|DrawGuides (Variables|Default|GetCurrentLoopIndex))))
    (:then_4
      (if (Variables|DefaultMesh|GetAutoFillEmptyMesh)
        (Variables|DefaultMesh|SetAutoFillEmptyMesh false)
        (for _index_2 (range 0 (- (Variables|Default|GetNumberOfSplinePoints) 1))
          (if (== (.trackmesh (Utilities|Array|Get(acopy) _splinepointarray_2 _index_2)) 0)
            (Utilities|Array|SetArrayElem _splinepointarray_2 _index_2 (Utilities|Struct|MakeSplinePoint_Struct (Variables|DefaultMesh|GetDefaultTrackMesh) (.width (Utilities|Array|Get(acopy) _splinepointarray_2 _index_2)) (.height (Utilities|Array|Get(acopy) _splinepointarray_2 _index_2))))))))))

(fn InitSpline
  (params (PointIndex :type Integer))
  (LocalVariables|SetLocalCurrentLoopIndex PointIndex)
  (LocalVariables|SetLocalNextLoopIndex (Math|Integer|%(Integer) (+ PointIndex 1) (Variables|Default|GetNumberOfSplinePoints)))
  (Utilities|FlowControl|Sequence
    (:then_0
      (LocalVariables|SetLocalStartLocation (.Location (Spline|GetLocationandTangentatSplinePoint (Variables|Default|GetSpline) (LocalVariables|GetLocalCurrentLoopIndex) "Local")))
      (LocalVariables|SetLocalStartTangent (.Tangent (Spline|GetLocationandTangentatSplinePoint (Variables|Default|GetSpline) (LocalVariables|GetLocalCurrentLoopIndex) "Local")))
      (LocalVariables|SetLocalEndLocation (.Location (Spline|GetLocationandTangentatSplinePoint (Variables|Default|GetSpline) (LocalVariables|GetLocalNextLoopIndex) "Local")))
      (LocalVariables|SetLocalEndTangent (.Tangent (Spline|GetLocationandTangentatSplinePoint (Variables|Default|GetSpline) (LocalVariables|GetLocalNextLoopIndex) "Local")))
      (LocalVariables|SetStartAngleMesh (Math|Trig|DegreesToRadians (.roll (Spline|GetRotationatSplinePoint (Variables|Default|GetSpline) (LocalVariables|GetLocalCurrentLoopIndex) "Local"))))
      (LocalVariables|SetLocalStartScale (Math|Vector2D|MakeVector2D (.width (Utilities|Array|Get(acopy) (Variables|Default|GetSplinePointArray) (LocalVariables|GetLocalCurrentLoopIndex))) (.height (Utilities|Array|Get(acopy) (Variables|Default|GetSplinePointArray) (LocalVariables|GetLocalCurrentLoopIndex)))))
      (LocalVariables|SetEndAngleMesh (Math|Trig|DegreesToRadians (.roll (Spline|GetRotationatSplinePoint (Variables|Default|GetSpline) (LocalVariables|GetLocalNextLoopIndex) "Local"))))
      (LocalVariables|SetLocal_EndScale (Math|Vector2D|MakeVector2D (.width (Utilities|Array|Get(acopy) (Variables|Default|GetSplinePointArray) (LocalVariables|GetLocalNextLoopIndex))) (.height (Utilities|Array|Get(acopy) (Variables|Default|GetSplinePointArray) (LocalVariables|GetLocalNextLoopIndex))))))
    (:then_1
      (bind _returnvalue (AddComponent|AddSplineMeshComponent false))
      (Collision|SetCollisionEnabled _returnvalue (Variables|Default|GetCollision))
      (Components|StaticMesh|SetStaticMesh _returnvalue (.trackmesh (Utilities|Array|Get(acopy) (Variables|Default|GetSplinePointArray) (LocalVariables|GetLocalCurrentLoopIndex))))
      (SplineMesh|SetStartandEnd _returnvalue (LocalVariables|GetLocalStartLocation) (LocalVariables|GetLocalStartTangent) (LocalVariables|GetLocalEndLocation) (LocalVariables|GetLocalEndTangent) true :!class /Script/Engine.SplineMeshComponent)
      (Class|SplineMeshComponent|SetStartRoll _returnvalue (LocalVariables|GetStartAngleMesh) true)
      (Class|SplineMeshComponent|SetEndRoll _returnvalue (LocalVariables|GetEndAngleMesh) true)
      (SplineMesh|SetStartScale _returnvalue (LocalVariables|GetLocalStartScale) true :!class /Script/Engine.SplineMeshComponent)
      (SplineMesh|SetEndScale _returnvalue (LocalVariables|GetLocal_EndScale) true :!class /Script/Engine.SplineMeshComponent))))

(fn DrawPointNumber
  (params (PointIndex :type Integer))
  (bind _spline (Variables|Default|GetSpline))
  (bind _returnvalue (Spline|GetLocationatSplinePoint _spline PointIndex "Local"))
  (if (Variables|Default|GetDrawTrackPointNumber)
    (bind _returnvalue_2 (AddComponent|AddTextRenderComponent false (Math|Transform|MakeTransform (Math|Vector|MakeVector (.x _returnvalue) (.y _returnvalue) (+ (.z _returnvalue) 5e+01)) (Spline|GetRotationatSplinePoint _spline PointIndex "Local"))))
    (Rendering|Components|TextRender|SetText _returnvalue_2 (Utilities|Text|ToText(Integer) PointIndex))
    (Rendering|Components|TextRender|SetWorldSize _returnvalue_2 1e+02)
    (Rendering|Components|TextRender|SetTextRenderColor _returnvalue_2 (Variables|Default|GetTrackPointNumberColor))
    (Development|SetHiddeninGame _returnvalue_2 (not (Variables|Default|GetDrawTrackPointNumber)) false)))

(fn DrawGuides
  (params (PointIndex :type Integer))
  (bind _spline (Variables|Default|GetSpline))
  (bind _returnvalue (Spline|GetLocationatSplinePoint _spline PointIndex "Local"))
  (if (Variables|Default|GetDrawTrackGuides)
    (bind _returnvalue_2 (AddComponent|AddArrowComponent false (Math|Transform|MakeTransform (Math|Vector|MakeVector (.x _returnvalue) (.y _returnvalue) (.z _returnvalue)) (Math|Conversions|RotationFromXVector (Math|Vector|GetUpVector (Spline|GetRotationatSplinePoint _spline PointIndex "Local"))) "2.500000,1,1.000000")))
    (Components|Arrow|SetArrowColor(LinearColor) _returnvalue_2 (Math|Conversions|ToLinearColor(Color) (Variables|Default|GetTrackPointNumberColor)))
    (Development|SetHiddeninGame _returnvalue_2 (not (Variables|Default|GetDrawTrackGuides)) false)))