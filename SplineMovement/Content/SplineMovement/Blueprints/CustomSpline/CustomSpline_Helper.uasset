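; CustomSpline_Helper is a set of utility functions for enemy control and character animation in the spline movement feature.
; It looks up the first actor with a given tag as an EnemyGenerator_BP, returning a found flag, and can destroy every EnemyCharacter_BP.
; It also overrides a third-person character's animation speed by writing the manual flag and speed into its ThirdPerson_AnimBP.
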(fn GetEnemyGeneratorbyTag
  (params (EnemyGeneratorName :type Name))
  (bind _outactors (Actor|GetAllActorswithTag 0 EnemyGeneratorName))
  (for _array_element _outactors
    (bind _asenemy_generator_bp (Utilities|Casting|CastToEnemyGenerator_BP _array_element))
    (return _asenemy_generator_bp true))
  (return 0 false))

(fn DestroyAllEnemy
  (bind _outactors (Actor|GetAllActorsOfClass 0 "/Game/SplineMovement/DemoContent/ThirdPerson/Blueprints/EnemyCharacter_BP.EnemyCharacter_BP_C"))
  (for _array_element _outactors
    (Actor|DestroyActor _array_element)))

(fn SetCharacterManualSpeed
  (params (ThirdPersonCharacter :type Third%20Person%20Character%20BP%20Object%20Reference) (Speed :type Float%20%28single-precision%29) (isSpeedManual :type Boolean))
  (bind _asthird_person_anim_bp (Utilities|Casting|CastToThirdPerson_AnimBP (Components|SkeletalMesh|GetAnimInstance (Variables|/Script/Engine.Character|GetMesh ThirdPersonCharacter))))
  (Variables|/Game/SplineMovement/DemoContent/ThirdPerson/Animations/ThirdPerson_AnimBP.ThirdPerson_AnimBP_C|SetisSpeedManual _asthird_person_anim_bp isSpeedManual)
  (Variables|/Game/SplineMovement/DemoContent/ThirdPerson/Animations/ThirdPerson_AnimBP.ThirdPerson_AnimBP_C|SetSpeed _asthird_person_anim_bp Speed))