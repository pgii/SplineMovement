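; EnemyGenerator_BP is a spawner that creates a batch of EnemyCharacter_BP AI pawns at random points inside its SpawnPlace box.
; GenerateEnemy re-arms a timer on itself with a random one-to-two-second interval, spawning one enemy per call until EnemyCount is reached.
; It then pauses the timer and resets the counter; nothing in this Blueprint starts the event.
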(event Custom|GenerateEnemy
  (bind _spawnplace (Variables|Default|GetSpawnPlace))
  (bind _returnvalue (Utilities|Time|SetTimerbyEvent (delegate Custom|GenerateEnemy) (Math|Random|RandomFloatinRange 1.0 2.0) true))
  (if (< (Variables|Default|GetEnemyGenerateComplete) (Variables|Default|GetEnemyCount))
    (AI|SpawnAIFromClass "/Game/SplineMovement/DemoContent/ThirdPerson/Blueprints/EnemyCharacter_BP.EnemyCharacter_BP_C" 0 (Math|Random|RandomPointinBoundingBox (Transformation|GetWorldLocation _spawnplace) (Components|Box|GetScaledBoxExtent _spawnplace)) "0, 0, 0" false)
    (Variables|Default|SetEnemyGenerateComplete (+ (Variables|Default|GetEnemyGenerateComplete) 1))
    (else
      (Utilities|Time|PauseTimerbyHandle _returnvalue)
      (Variables|Default|SetEnemyGenerateComplete 0))))

(fn ConstructionScript)