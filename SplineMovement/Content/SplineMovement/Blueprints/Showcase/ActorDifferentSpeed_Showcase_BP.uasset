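; Showcase actor that moves a platform along a custom spline at a different speed on each segment, looping indefinitely from BeginPlay.
; Chained MovePlatformSpline calls each cover a range of spline points and start the next on Completed.
; Start and end speeds match between segments, rising in steps before the last segment returns to the initial speed and restarts the cycle.
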(event EventBeginPlay
  (Utilities|MovePlatformSpline (Variables|Default|GetMovingPlatform) (Variables|Default|GetCustomSpline) 0 5e+01 2 2e+02 false false :!label _label
    (:Completed
      (Utilities|MovePlatformSpline (Variables|Default|GetMovingPlatform) (Variables|Default|GetCustomSpline) 2 2e+02 4 4e+02 false false
        (:Completed
          (Utilities|MovePlatformSpline (Variables|Default|GetMovingPlatform) (Variables|Default|GetCustomSpline) 4 4e+02 6 8e+02 false false
            (:Completed
              (Utilities|MovePlatformSpline (Variables|Default|GetMovingPlatform) (Variables|Default|GetCustomSpline) 6 8e+02 0 5e+01 false false
                (:Completed
                  (goto _label))))))))))

(fn ConstructionScript)