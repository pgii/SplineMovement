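; Showcase actor that moves a platform along a custom spline in timed point-to-point segments.
; On BeginPlay it chains MovePlatformSpline calls over successive point ranges (0→2→4→6→back to start) at constant speed.
; Each Completed callback waits one second before starting the next leg, and the last leg loops back to the first, so the cycle runs indefinitely.
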(event EventBeginPlay
  (Utilities|MovePlatformSpline (Variables|Default|GetMovingPlatform) (Variables|Default|GetCustomSpline) 0 2e+02 2 2e+02 false false :!label _label
    (:Completed
      (Utilities|FlowControl|Delay 1.0)
      (Utilities|MovePlatformSpline (Variables|Default|GetMovingPlatform) (Variables|Default|GetCustomSpline) 2 2e+02 4 2e+02 false false
        (:Completed
          (Utilities|FlowControl|Delay 1.0)
          (Utilities|MovePlatformSpline (Variables|Default|GetMovingPlatform) (Variables|Default|GetCustomSpline) 4 2e+02 6 2e+02 false false
            (:Completed
              (Utilities|FlowControl|Delay 1.0)
              (Utilities|MovePlatformSpline (Variables|Default|GetMovingPlatform) (Variables|Default|GetCustomSpline) 6 2e+02 0 2e+02 false false
                (:Completed
                  (Utilities|FlowControl|Delay 1.0)
                  (goto _label))))))))))

(fn ConstructionScript)