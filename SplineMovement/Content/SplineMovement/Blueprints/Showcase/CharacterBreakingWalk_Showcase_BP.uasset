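; Showcase actor that demonstrates interrupting and resuming a character's walk along a custom spline.
; The walkCharacterSpline node starts on BeginPlay and restarts after a zero-length delay whenever it completes, unless an IsBreaked flag marks an interruption.
; The player entering TriggerBox breaks the walk and sets MoveToCharacterEnable on the walking ShowcaseCharacter_BP.
; Leaving the box clears that flag and re-enters the spline walk.
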(event OnActorBeginOverlap(TriggerBox)
  (params (OverlappedActor :type Actor%20Object%20Reference) (OtherActor :type Actor%20Object%20Reference))
  (if (== OtherActor (Game|GetPlayerCharacter 0))
    (bind _asshowcase_character_bp (Utilities|Casting|CastToShowcaseCharacter_BP (Variables|Default|GetThirdPersonCharacter)))
    (Variables|/Game/SplineMovement/DemoContent/ThirdPerson/Blueprints/ShowcaseCharacter_BP.ShowcaseCharacter_BP_C|SetMoveToCharacterEnable _asshowcase_character_bp true)
    (Utilities|WalkCharacterSpline (Variables|Default|GetThirdPersonCharacter) (Variables|Default|GetCustomSpline) 5e+02 0 0 5e+02 0.0 true (Variables|Default|GetDistanceAlongSpline) false true false) ; enters at Break
  ))

(event OnActorEndOverlap(TriggerBox)
  (params (OverlappedActor :type Actor%20Object%20Reference) (OtherActor :type Actor%20Object%20Reference))
  (if (== OtherActor (Game|GetPlayerCharacter 0))
    (bind _asshowcase_character_bp (Utilities|Casting|CastToShowcaseCharacter_BP (Variables|Default|GetThirdPersonCharacter)))
    (Variables|/Game/SplineMovement/DemoContent/ThirdPerson/Blueprints/ShowcaseCharacter_BP.ShowcaseCharacter_BP_C|SetMoveToCharacterEnable _asshowcase_character_bp false)
    (Utilities|WalkCharacterSpline (Variables|Default|GetThirdPersonCharacter) (Variables|Default|GetCustomSpline) 5e+02 0 0 5e+02 0.0 true (Variables|Default|GetDistanceAlongSpline) false true false :!label _label
      (:Completed
        (if (stale _output_get)
          (Variables|Default|SetisBreaked false)
          (else
            (Utilities|FlowControl|Delay 0.0)
            (goto _label))))
      (:Breaked
        (bind _output_get (Variables|Default|SetisBreaked true))))))

(event EventBeginPlay
  (Utilities|WalkCharacterSpline (Variables|Default|GetThirdPersonCharacter) (Variables|Default|GetCustomSpline) 5e+02 0 0 5e+02 0.0 true (Variables|Default|GetDistanceAlongSpline) false true false :!label _label
    (:Completed
      (if (stale _output_get)
        (Variables|Default|SetisBreaked false)
        (else
          (Utilities|FlowControl|Delay 0.0)
          (goto _label))))
    (:Breaked
      (bind _output_get (Variables|Default|SetisBreaked true)))))

(fn ConstructionScript)