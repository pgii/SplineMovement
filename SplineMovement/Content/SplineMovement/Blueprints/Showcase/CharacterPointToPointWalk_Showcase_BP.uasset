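; Showcase Blueprint that walks a third-person character along a custom spline in point-to-point segments.
; On BeginPlay it chains four latent WalkCharacterSpline calls over successive point index ranges, with controller rotation and stop-after-finishing enabled.
; Each completion triggers a one-second pause before the next segment, and the last one loops back to the first for continuous movement.
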(event EventBeginPlay
  (Utilities|WalkCharacterSpline (Variables|Default|GetThirdPersonCharacter) (Variables|Default|GetCustomSpline) 5e+02 0 3 5e+02 0.0 true (Variables|Default|GetDistanceAlongSpline) false true false :!label _label
    (:Completed
      (Utilities|FlowControl|Delay 1.0)
      (Utilities|WalkCharacterSpline (Variables|Default|GetThirdPersonCharacter) (Variables|Default|GetCustomSpline) 5e+02 3 5 5e+02 0.0 true (Variables|Default|GetDistanceAlongSpline) false true false
        (:Completed
          (Utilities|FlowControl|Delay 1.0)
          (Utilities|WalkCharacterSpline (Variables|Default|GetThirdPersonCharacter) (Variables|Default|GetCustomSpline) 5e+02 5 7 5e+02 0.0 true (Variables|Default|GetDistanceAlongSpline) false true false
            (:Completed
              (Utilities|FlowControl|Delay 1.0)
              (Utilities|WalkCharacterSpline (Variables|Default|GetThirdPersonCharacter) (Variables|Default|GetCustomSpline) 5e+02 7 0 5e+02 0.0 true (Variables|Default|GetDistanceAlongSpline) false true false
                (:Completed
                  (Utilities|FlowControl|Delay 1.0)
                  (goto _label))))))))))

(fn ConstructionScript)