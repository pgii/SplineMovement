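; Demo Blueprint that, on BeginPlay, moves the player's third-person character along a spline in two chained segments.
; The WalkCharacterSpline macro snaps the character to a start point, then advances it each tick through a zero-Delay loop, easing speed toward an end speed.
; It follows spline XY and rotation, keeps the character's own Z, and fires Completed within a tolerance of the end point.
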(event EventBeginPlay
  (bind _customspline (Variables|Default|GetCustomSpline))
  (Utilities|FlowControl|Sequence
    (:then_1
      (Utilities|Casting|CastToThirdPersonCharacter_BP (Game|GetPlayerCharacter 0)))
    (:then_2
      (bind _asthird_person_character_bp (Utilities|Casting|CastToThirdPersonCharacter_BP (Game|GetPlayerCharacter 0)))
      (Utilities|WalkCharacterSpline _asthird_person_character_bp _customspline 5e+02 1 0.0 2 5e+02
        (:Completed
          (Utilities|WalkCharacterSpline _asthird_person_character_bp _customspline 2e+02 2 5e+02 3 1.5e+02))))))

(fn ConstructionScript)